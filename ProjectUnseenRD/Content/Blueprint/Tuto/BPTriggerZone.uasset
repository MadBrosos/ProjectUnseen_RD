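; Trigger zone in the Tuto folder that spawns a BP_FakeUnseen when the player walks in holding an object.
; Box overlap casts to BP_FirstPersonCharacter_CP and requires a valid ObjectHeld, which debug text calls an apple, though its type is unchecked.
; The spawn point lies a fixed distance along the player capsule's forward vector, with zero rotation.
; A Triggered flag limits it to one spawn, and debug prints report each outcome.
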(event OnComponentBeginOverlap(Box)
  (params (OverlappedComponent :type Primitive%20Component%20Object%20Reference) (OtherActor :type Actor%20Object%20Reference) (OtherComp :type Primitive%20Component%20Object%20Reference) (OtherBodyIndex :type Integer) (bFromSweep :type Boolean) (SweepResult :type Hit%20Result%20Structure%20%28by%20ref%29))
  (bind _asbp_first_person_character_cp (Utilities|Casting|CastToBP_FirstPersonCharacter_CP OtherActor)
    (:then
      (Utilities|IsValid (Variables|/Game/Blueprint/FirstPerson_Camera/BP_FirstPersonCharacter_CP.BP_FirstPersonCharacter_CP_C|GetObjectHeld _asbp_first_person_character_cp)
        (:Is%20Valid
          (if (Variables|Default|GetTriggered)
            (Development|PrintString "Already Triggered")
            (else
              (Development|PrintString "Spawn Unseen")
              (CallFunction|SpawnFakeUnseen _asbp_first_person_character_cp)
              (Variables|Default|SetTriggered true))))
        (:Is%20Not%20Valid
          (Development|PrintString "player doesnt hold apple"))))
    (:CastFailed
      (Development|PrintString "Cast To BP_FPSChar failed by BPTriggerZone" true true "(R=1.000000,G=0.043376,B=0.000000,A=1.000000)"))))

(event Custom|SpawnFakeUnseen
  (params (Char :type BP%20First%20Person%20Character%20CP%20Object%20Reference))
  (bind _unseentransforme (CallFunction|CreateNewTransform Char))
  (Game|SpawnActorfromClass :Class "/Game/Blueprint/PlaceHolder/BP_FakeUnseen.BP_FakeUnseen_C" :SpawnTransform _unseentransforme :CollisionHandlingOverride "Undefined" :TransformScaleMethod "MultiplyWithRoot" :Instigator 0))

(fn ConstructionScript)

(fn CreateNewTransform
  (params (Player :type BP%20First%20Person%20Character%20CP%20Object%20Reference))
  (bind _returnvalue (Transformation|GetActorLocation Player))
  (return (Math|Transform|MakeTransform (+ (Math|Vector|MakeVector (.x _returnvalue) (.y _returnvalue) (.z _returnvalue)) (* (Math|Vector|GetForwardVector (Variables|/Script/Engine.Character|GetCapsuleComponent Player)) 500)))))