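; BP_Cube is a cube actor that appears and disappears through a material dissolve effect.
; Its construction script creates a dynamic instance of MDissolve, applies it to the cube and sets an initial Progress value.
; The UnseenApear and UnseenDisapear events play and reverse one shared timeline, whose track drives the Progress parameter.
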(event Custom|UnseenDisapear
  (bind _newtrack_0 (Timeline|Timeline Reverse)
    (:Update
      (Rendering|Material|SetScalarParameterValue (Variables|Default|GetMID_Dissolve) "Progress" _newtrack_0 :!class /Script/Engine.MaterialInstanceDynamic))))

(event Custom|UnseenApear
  (bind _newtrack_0 (Timeline|Timeline Play)
    (:Update
      (Rendering|Material|SetScalarParameterValue (Variables|Default|GetMID_Dissolve) "Progress" _newtrack_0 :!class /Script/Engine.MaterialInstanceDynamic))))

(fn ConstructionScript
  (bind _returnvalue (Rendering|Material|CreateDynamicMaterialInstance (Variables|Default|GetMDissolve) "MID_Mat" "None" :!class /Script/Engine.KismetMaterialLibrary))
  (bind _output_get (Variables|Default|SetMID_Dissolve _returnvalue))
  (Rendering|Material|SetMaterial (Variables|Default|GetCube) 0 _output_get)
  (Rendering|Material|SetScalarParameterValue _output_get "Progress" 1.0 :!class /Script/Engine.MaterialInstanceDynamic))