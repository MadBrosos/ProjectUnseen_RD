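; BP_UnseenController is the AI controller for the Unseen, starting its BT_Unseen behavior tree on BeginPlay.
; AI Perception updates feed the Blackboard: sensed BPI_PickUp actors become Food, while other actors set targetActor and LastSeenPosition.
; Losing a pickup clears Food and prints a debug message; losing any other actor leaves its Blackboard values untouched.
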(event OnTargetPerceptionUpdated(AIPerception)
  (params (Actor :type Actor%20Object%20Reference) (Stimulus :type AI%20Stimulus%20Structure))
  (bind _blackboard (Variables|Default|GetBlackboard))
  (if (.bSuccessfullySensed (Utilities|Struct|BreakAIStimulus Stimulus))
    ;[1 1 1] Entered Sight
    (Utilities|Casting|CastToBPI_PickUp Actor
      (:then
        (AI|Components|Blackboard|SetValueasObject (Variables|Default|GetBlackboard) (Utilities|Name|MakeLiteralName "Food") Actor))
      (:CastFailed
        (AI|Components|Blackboard|SetValueasObject _blackboard (Utilities|Name|MakeLiteralName "targetActor") Actor)
        (AI|Components|Blackboard|SetValueasVector _blackboard (Utilities|Name|MakeLiteralName "LastSeenPosition") (Transformation|GetActorLocation Actor))))
    (else
      (Utilities|Casting|CastToBPI_PickUp Actor)
      (AI|Components|Blackboard|SetValueasObject (Variables|Default|GetBlackboard) (Utilities|Name|MakeLiteralName "Food") 0)
      (Development|PrintString "AppleLost"))))

(event EventBeginPlay
  (AI|RunBehaviorTree "/Game/AI/BT_Unseen.BT_Unseen"))

(fn ConstructionScript)