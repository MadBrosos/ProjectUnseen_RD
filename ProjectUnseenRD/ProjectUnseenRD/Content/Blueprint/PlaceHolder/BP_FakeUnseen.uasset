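; BP_FakeUnseen is a placeholder stand-in for the Unseen creature that performs a scripted theft of the player's held object.
; On BeginPlay, a timeline lerps it in front of the player, where it attaches the object to its anchor and calls SetCameraOn.
; A second timeline makes it flee back past its start point.
; After a delay, it triggers the object's pickup Action, spawns a controller-possessed A_Creature_Base in its place and destroys itself.
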(event Custom|StealObject
  (bind _capsulecomponent (Variables|Default|GetCapsuleComponent))
  (bind _player (Variables|Default|GetPlayer))
  (bind _returnvalue (Transformation|GetWorldTransform _capsulecomponent))
  (bind _output_get (Variables|Default|Setobject%20held (Variables|/Game/Blueprint/FirstPerson_Camera/BP_FirstPersonCharacter_CP.BP_FirstPersonCharacter_CP_C|GetObjectHeld _player)))
  (Transformation|AttachComponentToComponent _output_get (Variables|Default|GetAnchorPoint) "None" "SnapToTarget" "SnapToTarget" "KeepWorld" true)
  (Variables|/Game/Blueprint/FirstPerson_Camera/BP_FirstPersonCharacter_CP.BP_FirstPersonCharacter_CP_C|SetObjectHeld _player 0)
  (Default|SetCameraon _player)
  (Variables|Default|SetTargetPos (+ (Variables|Default|GetTargetPos) (* (- (Variables|Default|GetBasePos) (Variables|Default|GetTargetPos)) 5)))
  (Variables|Default|SetBasePos (Transformation|GetWorldLocation (Variables|Default|GetCapsuleComponent)))
  (bind _lerpvalue (Timeline|TimelineFlee PlayFromStart)
    (:Update
      (Transformation|SetActorLocation (Math|Vector|Lerp(Vector) (Variables|Default|GetBasePos) (Variables|Default|GetTargetPos) _lerpvalue) false false))
    (:Finished
      (Utilities|FlowControl|Delay 2.0)
      (bind _asbpi_pick_up (Utilities|Casting|CastToBPI_PickUp (Variables|Default|Getobject%20held)))
      (Default|Action _asbpi_pick_up)
      (bind _returnvalue_2 (Game|SpawnActorfromClass :Class "/Game/Blueprint/FirstPerson_Camera/A_Creature_Base.A_Creature_Base_C" :SpawnTransform _returnvalue :CollisionHandlingOverride "Undefined" :TransformScaleMethod "MultiplyWithRoot" :Instigator 0))
      (bind _returnvalue_3 (Game|SpawnActorfromClass "/Game/AI/BP_UnseenController.BP_UnseenController_C" _returnvalue "Undefined" "MultiplyWithRoot" 0 0))
      (Pawn|Possess _returnvalue_3 _returnvalue_2)
      (Actor|DestroyActor))))

(event EventBeginPlay
  (Variables|Default|SetBasePos (Transformation|GetWorldLocation (Variables|Default|GetCapsuleComponent)))
  (bind _returnvalue (Actor|GetActorOfClass "/Game/Blueprint/FirstPerson_Camera/BP_FirstPersonCharacter_CP.BP_FirstPersonCharacter_CP_C"))
  (Variables|Default|SetPlayer _returnvalue)
  (Variables|Default|SetTargetPos (+ (Transformation|GetActorLocation _returnvalue) (* (Math|Vector|GetForwardVector (Variables|/Script/Engine.Character|GetCapsuleComponent _returnvalue)) 250)))
  (bind _lerpvalue (Timeline|Timeline Play)
    (:Update
      (Transformation|SetActorLocation (Math|Vector|Lerp(Vector) (Variables|Default|GetBasePos) (Variables|Default|GetTargetPos) _lerpvalue) false false))
    (:Finished
      (CallFunction|StealObject))))

(fn ConstructionScript)