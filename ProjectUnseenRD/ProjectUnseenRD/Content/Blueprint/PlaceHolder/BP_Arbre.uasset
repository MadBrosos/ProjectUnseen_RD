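; BP_Arbre is a placeholder tree actor that keeps one apple spawned on it.
; It spawns an AppleClass actor at the SpawnApple component's transform on BeginPlay and stores the reference.
; Tick runs through a five-second Delay, so it periodically checks that reference and spawns a replacement when the apple is no longer valid.
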(event Custom|Spawn%20Apple%20Event
  (bind _returnvalue (Game|SpawnActorfromClass (Variables|Default|GetAppleClass) (Transformation|GetWorldTransform (Variables|Default|GetSpawnApple)) "Undefined" "MultiplyWithRoot" 0 0))
  (Variables|Default|SetApple _returnvalue))

(event EventBeginPlay
  (CallFunction|SpawnAppleEvent))

(event EventTick
  (params (DeltaSeconds :type Float%20%28single-precision%29))
  (Utilities|FlowControl|Delay 5.0)
  (Utilities|IsValid (Variables|Default|GetApple)
    (:Is%20Not%20Valid
      (CallFunction|SpawnAppleEvent))))

(fn ConstructionScript)