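; BP_Fruit is a fruit pickup actor that can be picked up, dropped and used.
; Pickup and Drop toggle physics simulation on its Sphere mesh, while Action destroys the actor; each prints a debug string.
; The construction script calls SetupFruits to fill FruitData from the fruit's name, mesh and fruit flag.
; Tick destroys the fruit once it falls below a kill height.
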(event EventTick
  (params (DeltaSeconds :type Float%20%28single-precision%29))
  (if (< (.z (Transformation|GetWorldLocation (Variables|Default|GetSphere))) -1e+03)
    (Actor|DestroyActor)))

(event EventAction
  (Development|PrintString "apple Action")
  (Actor|DestroyActor))

(event EventPickup
  (Physics|SetSimulatePhysics (Variables|Default|GetSphere) false)
  (Development|PrintString "pickup"))

(event EventDrop
  (Physics|SetSimulatePhysics (Variables|Default|GetSphere) true)
  (Development|PrintString "Drop"))

(fn ConstructionScript
  (CallFunction|SetupFruits))

(fn SetupFruits
  (Variables|Default|SetFruitData (Utilities|Struct|MakeST_PhotoCaptureInfo (Variables|Default|GetFruitName) (Variables|/Script/Engine.StaticMeshComponent|GetStaticMesh (Variables|Default|GetSphere)) 0 "0.000000,0.000000,0.000000|0.000000,0.000000,0.000000|1.000000,1.000000,1.000000" false (Variables|Default|GetFruit%20Data%20Is%20Fruit))))